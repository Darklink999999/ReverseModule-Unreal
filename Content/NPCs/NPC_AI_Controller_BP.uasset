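; AI controller for NPCs that runs the NPC behavior tree and pauses it when the player comes close.
; Each tick it checks distance to the player pawn; within range it stops the tree logic, turns the NPC to face the player and registers it as the nearby NPC in the game instance.
; When that registered NPC's player moves out of range, it restarts the tree and clears the near flag.
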(event `self.ReceiveBeginPlay`
  (`self.RunBehaviorTree` "/Game/NPCs/NPC_BT.NPC_BT"))

(event `self.ReceiveTick`
  (params (DeltaSeconds :type "Float (single-precision)"))
  (bind _returnvalue (`self.K2_GetPawn`))
  (bind (_returnvalue_roll _returnvalue_pitch _returnvalue_yaw) (`KismetMathLibrary.BreakRotator` (`KismetMathLibrary.Conv_VectorToRotator` (`KismetMathLibrary.Normal` (- (`self.K2_GetActorLocation` (`GameplayStatics.GetPlayerPawn` 0)) (`self.K2_GetActorLocation` (`self.K2_GetPawn`)))))))
  (if (<= (`KismetMathLibrary.Vector_Distance` (`self.K2_GetActorLocation` (`self.K2_GetPawn`)) (`self.K2_GetActorLocation` (`GameplayStatics.GetPlayerPawn` 0))) 250.0)
    (`BrainComponent.StopLogic` (`self.BrainComponent`) "NearPlayer")
    (`self.K2_SetActorRotation` _returnvalue (`KismetMathLibrary.MakeRotator` 0.0 0.0 _returnvalue_yaw) false)
    (bind _asgame_instance_bp (cast `/Game/ThirdPersonBP/Maps/GameInstance_BP` (`GameplayStatics.GetGameInstance`)))
    (set `/Game/ThirdPersonBP/Maps/GameInstance_BP.nearNPC` true _asgame_instance_bp)
    (set `/Game/ThirdPersonBP/Maps/GameInstance_BP.npcThatIsNear` _returnvalue _asgame_instance_bp)
    (else
      (bind _asgame_instance_bp_2 (cast `/Game/ThirdPersonBP/Maps/GameInstance_BP` (`GameplayStatics.GetGameInstance`)))
      (if (and (`/Game/ThirdPersonBP/Maps/GameInstance_BP.nearNPC` _asgame_instance_bp_2) (== (`/Game/ThirdPersonBP/Maps/GameInstance_BP.npcThatIsNear` _asgame_instance_bp_2) (`self.K2_GetPawn`)))
        (`self.RunBehaviorTree` "/Game/NPCs/NPC_BT.NPC_BT")
        (bind _asgame_instance_bp_3 (cast `/Game/ThirdPersonBP/Maps/GameInstance_BP` (`GameplayStatics.GetGameInstance`)))
        (set `/Game/ThirdPersonBP/Maps/GameInstance_BP.nearNPC` false _asgame_instance_bp_3)))))

(fn `UserConstructionScript`)